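; BP_Note is a moving note actor, apparently for a rhythm mechanic, that travels in a straight line until hit.
; On BeginPlay it snaps to StartLocation and caches the normalized vector from HitLocation to itself as Direction.
; Tick advances it along Direction by NoteSpeed scaled by delta time while HasBeenHit is false, so positive speed moves it away from HitLocation.
; HasBeenHit is only read here, and SpawnTime is unused.
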(event `self.ReceiveBeginPlay`
  (`self.K2_SetActorLocation` (`self.StartLocation`))
  (set `self.Direction` (`KismetMathLibrary.Normal` (- (`self.K2_GetActorLocation`) (`self.HitLocation`)))))

(event `self.ReceiveTick`
  (params (DeltaSeconds :type "Float (single-precision)"))
  (if (not (`self.HasBeenHit`))
    (`self.K2_SetActorLocation` (+ (`self.K2_GetActorLocation`) (* (`self.Direction`) (`self.NoteSpeed`) DeltaSeconds)))))

(fn `UserConstructionScript`)