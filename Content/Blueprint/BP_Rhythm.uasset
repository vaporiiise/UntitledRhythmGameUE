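; Rhythm game actor that plays an FMOD beatmap event and spawns notes from its timeline markers.
; Each marker prints its name, then randomly picks the left or right spawner to create a BP_Note.
; The note receives a fixed speed, a zero spawn time and start and hit points read from lane splines.
; Both sides take the hit point from the left lane, and the lane variables are cleared before use.
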(event `self.ReceiveBeginPlay`
  (bind _rhythmaudio (`self.RhythmAudio`))
  (`FMODAudioComponent.SetEvent` (`self.RhythmAudio`) "/Game/FMOD/Events/Beatmap.Beatmap")
  (`FMODAudioComponent.Play` _rhythmaudio)
  (`self.FmodMarkers` "")
  (add `FMODAudioComponent.OnTimelineMarker` _rhythmaudio (delegate `FMODMarkers`))
  (`self.FmodMarkers` ""))

(event `FMODMarkers`
  (params (Name :type String) (Position :type Integer))
  (`KismetSystemLibrary.PrintString` Name)
  (if (== (`KismetMathLibrary.RandomBool`) false)
    (set `self.Left Lane` null)
    (bind _returnvalue (`|SpawnActorFromClass` "/Game/Blueprint/BP_Note.BP_Note_C" (`SceneComponent.K2_GetComponentToWorld` (`self.Left Spawner`)) "Undefined" "MultiplyWithRoot" null null))
    (set `/Game/Blueprint/BP_Note.StartLocation` (`SplineComponent.GetLocationAtSplinePoint` (`self.Left Lane`) 0 "World") _returnvalue)
    (set `/Game/Blueprint/BP_Note.HitLocation` (`SplineComponent.GetLocationAtSplinePoint` (`self.Left Lane`) 1000 "World") _returnvalue)
    (set `/Game/Blueprint/BP_Note.NoteSpeed` 500.0 _returnvalue)
    (set `/Game/Blueprint/BP_Note.SpawnTime` 0.0 _returnvalue)
    (`FMODAudioComponent.GetTimelinePosition` (`self.RhythmAudio`))
    (else
      (set `self.Right Lane` null)
      (bind _returnvalue_2 (`|SpawnActorFromClass` "/Game/Blueprint/BP_Note.BP_Note_C" (`SceneComponent.K2_GetComponentToWorld` (`self.Right Spawner`)) "Undefined" "MultiplyWithRoot" null null))
      (set `/Game/Blueprint/BP_Note.StartLocation` (`SplineComponent.GetLocationAtSplinePoint` (`self.Right Lane`) 0 "World") _returnvalue_2)
      (set `/Game/Blueprint/BP_Note.HitLocation` (`SplineComponent.GetLocationAtSplinePoint` (`self.Left Lane`) 1000 "World") _returnvalue_2)
      (set `/Game/Blueprint/BP_Note.NoteSpeed` 500.0 _returnvalue_2)
      (set `/Game/Blueprint/BP_Note.SpawnTime` 0.0 _returnvalue_2)
      (`FMODAudioComponent.GetTimelinePosition` (`self.RhythmAudio`)))))

(fn `UserConstructionScript`)