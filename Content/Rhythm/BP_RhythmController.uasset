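; BP_RhythmController is a controller for the rhythm game that relays left and right hit events to the BP_Rhythm actors in the level.
; Hit_Left and Hit_Right each look up every BP_Rhythm actor and call its LaneHit with the lane name "Input A" or "Input D", respectively.
; On BeginPlay it hides the mouse cursor and enables input.
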(event `Hit_Left`
  (bind _outactors (`GameplayStatics.GetAllActorsOfClass` "/Game/Blueprint/BP_Rhythm.BP_Rhythm_C"))
  (for _array_element _outactors
    (bind _asbp_rhythm (cast `/Game/Blueprint/BP_Rhythm` _array_element))
    (`/Game/Blueprint/BP_Rhythm.LaneHit` _asbp_rhythm "Input A")))

(event `Hit_Right`
  (bind _outactors (`GameplayStatics.GetAllActorsOfClass` "/Game/Blueprint/BP_Rhythm.BP_Rhythm_C"))
  (for _array_element _outactors
    (bind _asbp_rhythm (cast `/Game/Blueprint/BP_Rhythm` _array_element))
    (`/Game/Blueprint/BP_Rhythm.LaneHit` _asbp_rhythm "Input D")))

(event `self.ReceiveBeginPlay`
  (set `self.bShowMouseCursor` false)
  (`self.EnableInput` null))

(fn `UserConstructionScript`)